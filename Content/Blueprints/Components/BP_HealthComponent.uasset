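; Health component that tracks an actor's health and alive state and broadcasts changes through event dispatchers.
; ChangeHealth subtracts damage and broadcasts the new value, but on lethal damage it clears IsAlive and fires the death event without updating Health.
; RefreshHealth restores full health, broadcasts it and starts a one-shot timer, likely to restore the alive flag via ChangeAliveParam after a short delay.
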(fn `ChangeAliveParam`
  (set `self.bIsAlive` true))

(fn `ChangeHealth`
  (params (Damage :type "Float (double-precision)"))
  (bind _returnvalue (- (`self.Health`) Damage))
  (if (<= _returnvalue 0.0)
    (set `self.bIsAlive` false)
    (`self.OnDeadEvent`)
    (else
      (bind _output_get (set `self.Health` _returnvalue))
      (`self.OnHealthChange` _output_get))))

(fn `RefreshHealth`
  (bind _output_get (set `self.Health` 100.0))
  (`self.OnHealthChange` _output_get)
  (`KismetSystemLibrary.K2_SetTimerDelegate` (`|CreateDelegate` :!event `ChangeAliveParam`) 5.0))