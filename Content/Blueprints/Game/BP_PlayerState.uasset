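; Player state that tracks the player's score and signals when the winning score is reached.
; On BeginPlay it copies the score-to-win threshold from BP_GameInstance.
; IncrementScore raises the score and broadcasts OnIncrementScore for the widget, then fires OnEndGame with true once the score meets or exceeds the threshold.
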(event `self.ReceiveBeginPlay`
  ;[1 1 1] Settings
  (bind _asbp_game_instance (cast `/Game/Blueprints/Game/BP_GameInstance` (`GameplayStatics.GetGameInstance`)))
  (set `self.ScoreToWin` (`/Game/Blueprints/Game/BP_GameInstance.ScoreToWin` _asbp_game_instance)))

(event `IncrementScore`
  (params (PlayerScore :type "Float (double-precision)"))
  ;[1 1 1] Increment
  (set `self.PlayerScore` (+ PlayerScore (`self.PlayerScore`)))
  ;[1 1 1] Dispatcher for widget
  (`self.OnIncrementScore` (`self.PlayerScore`))
  ;[1 1 1] Check condition to win
  (if (>= (`self.PlayerScore`) (`self.ScoreToWin`))
    (`self.OnEndGame` true)))

(fn `UserConstructionScript`)