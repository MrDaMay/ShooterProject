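; Player controller that creates the main UI, manages player lives and opens the pause or stop widget.
; On BeginPlay it adds BPW_UserInterface to the viewport and sets Game and UI input focused on it.
; TryToRespawn fires the life-change dispatcher and decrements PlayerLifes, then ends the game through BP_GameMode as a loss at zero or fires restart.
; Escape fires the stop-widget dispatcher.
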(event `self.ReceiveBeginPlay`
  (bind _returnvalue (`|CreateWidget` "/Game/Blueprints/Widgets/BPW_UserInterface.BPW_UserInterface_C"))
  (`UserWidget.AddToViewport` _returnvalue 0)
  (`WidgetBlueprintLibrary.SetInputMode_GameAndUIEx` self _returnvalue))

(event `TryToRespawn`
  (`self.OnIncrementLife`)
  (`/Engine/EditorBlueprintResources/StandardMacros.DecrementInt` (`self.PlayerLifes`)
    (:`  `
      (if (<= (`self.PlayerLifes`) 0)
        (bind _asbp_game_mode (cast `/Game/Blueprints/Game/BP_GameMode` (`GameplayStatics.GetGameMode`)))
        (`/Game/Blueprints/Game/BP_GameMode.EndGameEvent` _asbp_game_mode false)
        (else
          (`self.OnRestart`))))))

(event `Key|Escape` :paused true
  (params (Key :type "Key Structure"))
  (:`Pressed`
    (`self.OnOpenStopWidget`)))

(fn `UserConstructionScript`)