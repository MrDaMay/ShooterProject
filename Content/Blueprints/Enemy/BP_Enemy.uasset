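; BP_Enemy is an enemy character that makes random melee montage attacks, takes damage and dies.
; Attack locks re-attacking until the montage ends, and its "Attack" notify fires a debug-drawn forward sphere trace that damages the hit actor.
; Incoming damage goes to BPHealthComponent, whose dead event is bound at BeginPlay.
; DeadEvent stops movement and collision, plays a random death animation, updates BPKillScoreComponent and sets lifespan to the animation length.
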(event `self.ReceiveBeginPlay`
  (add `/Game/Blueprints/Components/BP_HealthComponent.OnDeadEvent` (`self.BP_HealthComponent`) (`|CreateDelegate` :!event `DeadEvent`)))

(event `self.ReceiveAnyDamage`
  (params (Damage :type "Float (single-precision)") (DamageType :type "DamageType Object Reference") (InstigatedBy :type "Controller Object Reference") (DamageCauser :type "Actor Object Reference"))
  (`/Game/Blueprints/Components/BP_HealthComponent.ChangeHealth` (`self.BP_HealthComponent`) Damage))

(event `/Game/Blueprints/Enemy/AI/BPI_Combat.Attack`
  (bind _returnvalue (`self.K2_GetActorLocation`))
  (bind _returnvalue_2 (`self.GetActorForwardVector`))
  (bind _attackmontages (`self.AttackMontages`))
  (`self.SetStateAttack` false)
  (bind _notifyname (`|PlayMontage` (`self.Mesh`) (`|GetArrayItem` _attackmontages (`KismetMathLibrary.RandomIntegerInRange` 0 (- (`KismetArrayLibrary.Array_Length` _attackmontages) 1))))
    (:`OnCompleted`
      (`self.SetStateAttack` true :!label _label))
    (:`OnInterrupted`
      (goto _label))
    (:`OnNotifyBegin`
      (if (== _notifyname "Attack")
        (bind _outhit (`KismetSystemLibrary.SphereTraceSingle` (+ _returnvalue (* _returnvalue_2 80)) (+ _returnvalue (* _returnvalue_2 120)) 50.0 "TraceTypeQuery3" false (`|MakeArray` self :!type "Actor Object Reference") "ForDuration"))
        (bind (_bblockinghit _binitialoverlap _time _distance _location _impactpoint _normal _impactnormal _physmat _hitactor) (`GameplayStatics.BreakHitResult` _outhit))
        (`/Engine/EditorBlueprintResources/StandardMacros.IsValid` _hitactor
          (:`Is Valid`
            (`GameplayStatics.ApplyDamage` _hitactor (`self.BaseDamage`) (`self.GetController`) self "/Script/Engine.DamageType")))))))

(fn `bIsAlive`
  (returns (bIsAlive :type Boolean))
  (return (`/Game/Blueprints/Components/BP_HealthComponent.bIsAlive` (`self.BP_HealthComponent`))))

(fn `CanAttack`
  (returns (bIsCanAttack :type Boolean))
  (return (`self.bIsCanAttack`)))

(fn `DeadEvent`
  (locals (Montage :type "AnimMontage Object Reference"))
  (bind _deathmontages (`self.DeathMontages`))
  ;[1 1 1] Stop moving
  (set `CharacterMovementComponent.MaxWalkSpeed` 0.0 (`self.CharacterMovement`))
  ;[1 1 1] Play random death montage
  (set `local.Montage` (`|GetArrayItem` _deathmontages (`KismetMathLibrary.RandomIntegerInRange` 0 (- (`KismetArrayLibrary.Array_Length` _deathmontages) 1))))
  (`SkeletalMeshComponent.PlayAnimation` (`self.Mesh`) (`local.Montage`) false)
  ;[1 1 1] Disable collision
  (`PrimitiveComponent.SetCollisionEnabled` (`self.CapsuleComponent`) "NoCollision")
  ;[1 1 1] Destroy after animation
  (`self.SetLifeSpan` (`AnimationAsset.GetPlayLength` (`local.Montage`)))
  ;[1 1 1] Increment score
  (`/Game/Blueprints/Components/BP_KillScoreComponent.Dead` (`self.BP_KillScoreComponent`)))

(fn `SetStateAttack`
  (params (bIsCanAttack :type Boolean))
  (set `self.bIsCanAttack` bIsCanAttack))

(fn `UserConstructionScript`)