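; BP_SpawnEnemy is a spawner actor that periodically spawns BP_Enemy at random points around its center, scaled from its Box extent.
; On BeginPlay it reads the enemy cap and spawn interval from BP_GameInstance, then waits briefly before starting a looping spawn timer.
; A counter limits spawns to the cap and drops whenever BP_PlayerState's score-increment event fires, freeing a slot for another enemy.
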(event `self.ReceiveBeginPlay`
  ;[1 1 1] Settings
  (bind _asbp_game_instance (cast `/Game/Blueprints/Game/BP_GameInstance` (`GameplayStatics.GetGameInstance`)))
  (set `self.MaxEnemyOnLevel` (`/Game/Blueprints/Game/BP_GameInstance.MaxEnemyOnLevel` _asbp_game_instance))
  (set `self.DelayForSpawnEnemy` (`/Game/Blueprints/Game/BP_GameInstance.DelayForSpawnEnemy` _asbp_game_instance))
  ;[1 1 1] Delay for widget
  (`KismetSystemLibrary.K2_SetTimerDelegate` (delegate `AfterDelay`) 2.0))

(event `AfterDelay`
  ;[1 1 1] Delay for widget
  (`KismetSystemLibrary.K2_SetTimerDelegate` (delegate `SpawnEnemy`) (`self.DelayForSpawnEnemy`) true)
  ;[1 1 1] Increment enemy for spawn
  (bind _asbp_player_state (cast `/Game/Blueprints/Game/BP_PlayerState` (`GameplayStatics.GetPlayerState` 0)))
  (add `/Game/Blueprints/Game/BP_PlayerState.OnIncrementScore` _asbp_player_state (delegate `IncrementEnemy`)))

(event `IncrementEnemy`
  (params (Score :type "Float (double-precision)"))
  ;[1 1 1] Increment enemy for spawn
  (`/Engine/EditorBlueprintResources/StandardMacros.DecrementInt` (`self.EnemyCout`)))

(event `SpawnEnemy`
  (bind (_returnvalue_x _returnvalue_y) (`KismetMathLibrary.BreakVector` (`BoxComponent.GetScaledBoxExtent` (`self.Box`))))
  ;[1 1 1] Check max enemy
  (if (< (`self.EnemyCout`) (`self.MaxEnemyOnLevel`))
    ;[1 1 1] Spawn and increment
    (`|SpawnActorFromClass` "/Game/Blueprints/Enemy/BP_Enemy.BP_Enemy_C" (`KismetMathLibrary.MakeTransform` (`KismetMathLibrary.RandomPointInBoundingBox` (`self.K2_GetActorLocation`) (`KismetMathLibrary.MakeVector` (/ _returnvalue_x 2.0) (/ _returnvalue_y 2.0)))) "AdjustIfPossibleButAlwaysSpawn" "OverrideRootScale" null null)
    (`/Engine/EditorBlueprintResources/StandardMacros.IncrementInt` (`self.EnemyCout`))))

(fn `UserConstructionScript`)