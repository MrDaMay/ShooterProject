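; BP_Weapon is a weapon actor that plays a fire animation and launches projectiles.
; On BeginPlay it casts its owner to BP_Character and binds to that character's OnFire event, so it relies on the owner to signal shots.
; Fire plays AM_Fire on the skeletal mesh, then SpawnProjectile always spawns a half-scale BP_Projectile at the Arrow component, facing along its forward vector.
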(event `self.ReceiveBeginPlay`
  (bind _asbp_character (cast `/Game/Blueprints/Character/BP_Character` (`self.GetOwner`)))
  (add `/Game/Blueprints/Character/BP_Character.OnFireEvent` _asbp_character (`|CreateDelegate` :!event `Fire`)))

(fn `Fire`
  (`SkeletalMeshComponent.PlayAnimation` (`self.SkeletalMesh`) "/Game/Blueprints/Weapon/Animations/AM_Fire.AM_Fire" false)
  (`self.SpawnProjectile`))

(fn `SpawnProjectile`
  (bind _arrow (`self.Arrow`))
  (bind _returnvalue (`SceneComponent.K2_GetComponentLocation` _arrow))
  (`|SpawnActorFromClass` "/Game/Blueprints/Weapon/BP_Projectile.BP_Projectile_C" (`KismetMathLibrary.MakeTransform` (`SceneComponent.K2_GetComponentLocation` (`self.Arrow`)) (`KismetMathLibrary.FindLookAtRotation` _returnvalue (+ _returnvalue (* (`SceneComponent.GetForwardVector` _arrow) 2000))) (0.5 0.5 0.5)) "AlwaysSpawn" "OverrideRootScale" null 0.0 null))

(fn `UserConstructionScript`)