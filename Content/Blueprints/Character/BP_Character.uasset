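; Player character for a cursor-aimed shooter: moves on input axes, faces the mouse and carries a spawned weapon on its hand socket.
; Tick applies movement, places a cursor decal under the mouse and yaws toward a mouse-ray/horizontal-plane intersection.
; Left mouse broadcasts OnFireEvent through a cooldown check and looping timer.
; Damage feeds the health component, whose death event requests a controller respawn; the controller's restart event refreshes health.
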(event `self.ReceiveBeginPlay`
  (bind _asbp_player_controller (cast `/Game/Blueprints/Game/BP_PlayerController` (`self.GetOwner`)))
  (bind _output_get (set `self.As BP Player Controller` _asbp_player_controller))
  ;[1 1 1] Refresh health
  (add `/Game/Blueprints/Game/BP_PlayerController.OnRestart` _output_get (delegate `Restart`))
  ;[1 1 1] Spawn decal
  (bind _returnvalue (`GameplayStatics.SpawnDecalAtLocation` "/Game/Cursor/M_Cursor.M_Cursor" (20.0 40.0 40.0)))
  (set `self.Cursor` _returnvalue)
  ;[1 1 1] Spawn and attach weapon
  (bind _returnvalue_2 (`|SpawnActorFromClass` "/Game/Blueprints/Weapon/BP_Weapon.BP_Weapon_C" (`KismetMathLibrary.MakeTransform` (0.0 0.0 0.0)) "AlwaysSpawn" "OverrideRootScale" self null))
  (`self.K2_AttachToComponent` _returnvalue_2 (`self.Mesh`) "WeaponSocket" "KeepRelative" "KeepRelative" "KeepRelative" true)
  ;[1 1 1] Dead event
  (add `/Game/Blueprints/Components/BP_HealthComponent.OnDeadEvent` (`self.BP_HealthComponent`) (delegate `DeadEvent`)))

(event `Restart`
  ;[1 1 1] Refresh health
  (`/Game/Blueprints/Components/BP_HealthComponent.RefreshHealth` (`self.BP_HealthComponent`)))

(event `DeadEvent`
  ;[1 1 1] Dead event
  (`/Game/Blueprints/Game/BP_PlayerController.TryToRespawn` (`self.As BP Player Controller`)))

(event `self.ReceiveTick`
  (params (DeltaSeconds :type "Float (single-precision)"))
  ;[1 1 1] Move
  (`self.AddMovementInput` (`KismetMathLibrary.MakeVector` (`self.MoveForward`) (`self.MoveRight`)))
  (`self.ChangeDecalCursorPosition`) ; Change decal position
  (`self.RotateCharacter`) ; Rotation character to cursor
  ;[1 1 1] Fire delay
  (set `self.TimerForFire` (+ DeltaSeconds (`self.TimerForFire`))))

(event `InputAxis|MoveRight`
  (params (AxisValue :type "Float (single-precision)"))
  ;[1 1 1] Movement event
  (set `self.MoveRight` AxisValue))

(event `InputAxis|MoveForward`
  (params (AxisValue :type "Float (single-precision)"))
  ;[1 1 1] Movement event
  (set `self.MoveForward` AxisValue))

(event `Key|LeftMouseButton`
  (params (Key :type "Key Structure"))
  ;[1 1 1] Fire
  (:`Pressed`
    (if (>= (`self.TimerForFire`) 0.3)
      (`self.Fire`))
    (bind _returnvalue (`KismetSystemLibrary.K2_SetTimerDelegate` (delegate `FireEvent`) 0.3 true))
    (set `self.FireTimer` _returnvalue))
  (:`Released`
    (`KismetSystemLibrary.K2_ClearAndInvalidateTimerHandle` (`self.FireTimer`))))

(event `FireEvent`
  ;[1 1 1] Fire
  (`self.Fire`))

(event `self.ReceiveAnyDamage`
  (params (Damage :type "Float (single-precision)") (DamageType :type "DamageType Object Reference") (InstigatedBy :type "Controller Object Reference") (DamageCauser :type "Actor Object Reference"))
  (`/Game/Blueprints/Components/BP_HealthComponent.ChangeHealth` (`self.BP_HealthComponent`) Damage))

(fn `ChangeDecalCursorPosition`
  (`SceneComponent.K2_SetWorldLocation` (`self.Cursor`) (`.Location` (`GameplayStatics.BreakHitResult` (`PlayerController.GetHitResultUnderCursorByChannel` (`self.As BP Player Controller`) "TraceTypeQuery1" true))) false false))

(fn `Fire`
  (`self.OnFireEvent`) ; Fire
  (set `self.TimerForFire` 0.0))

(fn `RotateCharacter`
  (bind (_worldlocation _worlddirection) (`PlayerController.DeprojectMousePositionToWorld` (`self.As BP Player Controller`)))
  (bind (_returnvalue_roll _returnvalue_pitch _returnvalue_yaw) (`KismetMathLibrary.BreakRotator` (`KismetMathLibrary.FindLookAtRotation` (`self.K2_GetActorLocation`) (`.Intersection` (`KismetMathLibrary.LinePlaneIntersection_OriginNormal` _worldlocation (+ _worldlocation (* _worlddirection 5000)) (`self.K2_GetActorLocation`) (0.0 0.0 1.0))))))
  (`self.K2_SetActorRotation` (`KismetMathLibrary.MakeRotator` 0.0 0.0 _returnvalue_yaw)))

(fn `UserConstructionScript`)